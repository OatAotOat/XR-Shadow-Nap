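; Interactive computer actor for VR that opens a quiz when the player activates it from nearby.
; Overlap of the VRPawn with BoxCollision enables input and shows Widget; leaving disables input and hides it.
; While input is enabled, either hand's point action swaps Widget for Quiz and plays a Windows XP startup sound at the actor.
; Leaving the box does not hide Quiz.
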(event OnComponentBeginOverlap(BoxCollision)
  (params (OverlappedComponent :type Primitive%20Component%20Object%20Reference) (OtherActor :type Actor%20Object%20Reference) (OtherComp :type Primitive%20Component%20Object%20Reference) (OtherBodyIndex :type Integer) (bFromSweep :type Boolean) (SweepResult :type Hit%20Result%20Structure%20%28by%20ref%29))
  (Utilities|Casting|CastToVRPawn OtherActor)
  (Input|EnableInput (Game|GetPlayerController 0))
  (Rendering|SetVisibility (Variables|Default|GetWidget) true false))

(event OnComponentEndOverlap(BoxCollision)
  (params (OverlappedComponent :type Primitive%20Component%20Object%20Reference) (OtherActor :type Actor%20Object%20Reference) (OtherComp :type Primitive%20Component%20Object%20Reference) (OtherBodyIndex :type Integer))
  (Utilities|Casting|CastToVRPawn OtherActor)
  (Input|DisableInput (Game|GetPlayerController 0))
  (Rendering|SetVisibility (Variables|Default|GetWidget) false false))

(event Input|EnhancedActionEvents|EnhancedInputActionIA_Hand_Point_Left
  (params (ActionValue :type Float%20%28double-precision%29) (ElapsedSeconds :type Float%20%28double-precision%29) (TriggeredSeconds :type Float%20%28double-precision%29) (InputAction :type Input%20Action%20Object%20Reference :default "/Game/VRTemplate/Input/Actions/Hands/IA_Hand_Point_Left.IA_Hand_Point_Left"))
  (:Started
    (Rendering|SetVisibility (Variables|Default|GetWidget) false false)
    (Rendering|SetVisibility (Variables|Default|GetQuiz) true false)
    (Audio|PlaySoundatLocation "/Game/Microsoft_Windows_XP_Startup_Sound.Microsoft_Windows_XP_Startup_Sound" (Transformation|GetActorLocation) "0, 0, 0" 1.0 1.0 0.0 0 0 0 0)))

(event Input|EnhancedActionEvents|EnhancedInputActionIA_Hand_Point_Right
  (params (ActionValue :type Float%20%28double-precision%29) (ElapsedSeconds :type Float%20%28double-precision%29) (TriggeredSeconds :type Float%20%28double-precision%29) (InputAction :type Input%20Action%20Object%20Reference :default "/Game/VRTemplate/Input/Actions/Hands/IA_Hand_Point_Right.IA_Hand_Point_Right"))
  (:Started
    (Rendering|SetVisibility (Variables|Default|GetWidget) false false)
    (Rendering|SetVisibility (Variables|Default|GetQuiz) true false)
    (Audio|PlaySoundatLocation "/Game/Microsoft_Windows_XP_Startup_Sound.Microsoft_Windows_XP_Startup_Sound" (Transformation|GetActorLocation) "0, 0, 0" 1.0 1.0 0.0 0 0 0 0)))

(fn ConstructionScript)