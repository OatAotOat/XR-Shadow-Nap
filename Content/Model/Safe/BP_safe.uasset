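; BP_safe is a safe with a keypad widget that opens its door when the correct code is entered.
; When the keypad widget component fires its released event, the entered code in KeyPad_UI is compared with CorrectCode.
; A match shows a success message, then after a delay snaps the door to an open position and rotation.
; A mismatch shows an error, then clears the display after a delay.
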(event OnReleased(KeypadWidget)
  (params (TouchedComponent :type Primitive%20Component%20Object%20Reference) (ButtonReleased :type Key%20Structure :default "None"))
  (bind _safedoor (Variables|Default|GetSafeDoor))
  (bind _askey_pad_ui (Utilities|Casting|CastToKeyPad_UI (UserInterface|GetUserWidgetObject (Variables|Default|GetKeypadWidget))))
  (if (Utilities|Enum|Equal(Enum) (Variables|/Game/Model/Safe/KeyPad_UI.KeyPad_UI_C|GetCurrentCode _askey_pad_ui) (Variables|Default|GetCorrectCode))
    (Variables|/Game/Model/Safe/KeyPad_UI.KeyPad_UI_C|SetCurrentCode _askey_pad_ui "Correct !")
    (Utilities|FlowControl|Delay 3.0)
    (Transformation|SetRelativeLocation _safedoor (Math|Vector|MakeVector 0.0 112.5 0.0) false false)
    (Transformation|SetRelativeRotation _safedoor "0.000000,90.000000,0.000000" false false)
    (else
      (Variables|/Game/Model/Safe/KeyPad_UI.KeyPad_UI_C|SetCurrentCode _askey_pad_ui "Wrong !")
      (Utilities|FlowControl|Delay 3.0)
      (Variables|/Game/Model/Safe/KeyPad_UI.KeyPad_UI_C|SetCurrentCode _askey_pad_ui ""))))

(fn ConstructionScript)