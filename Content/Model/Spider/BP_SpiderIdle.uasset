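; Spider actor that stays idle for a minute after BeginPlay, then makes its Hifispider component visible and moves it back and forth.
; Two timelines drive its relative Y location, one played forward and the other in reverse, with a 180-degree rotation flip between them.
; Each timeline triggers the other through a five-second Delay wired to Update rather than Finished, forming an endless loop.
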(event EventBeginPlay
  (bind _hi_fi_spider (Variables|Default|Gethi-fi-spider))
  (bind _hi_fi_spider_2 (Variables|Default|Gethi-fi-spider))
  (Utilities|FlowControl|Delay 6e+01)
  (Rendering|SetVisibility (Variables|Default|Gethi-fi-spider) true false)
  (bind _moveyaxis (Timeline|Timeline Play)
    (:Update
      (Transformation|SetRelativeRotation _hi_fi_spider "0, 0, 0" false false)
      (Transformation|SetRelativeLocation _hi_fi_spider (Math|Vector|MakeVector 0.0 _moveyaxis 0.0) false false)
      (Utilities|FlowControl|Delay 5.0)
      (bind _moveyaxis_2 (Timeline|Timeline_0 ReverseFromEnd)
        (:Update
          (Transformation|SetRelativeRotation _hi_fi_spider_2 "0.000000,180.000000,0.000000" false false)
          (Transformation|SetRelativeLocation _hi_fi_spider_2 (Math|Vector|MakeVector 0.0 _moveyaxis_2 0.0) false false)
          (Utilities|FlowControl|Delay 5.0)
          (Timeline|Timeline PlayFromStart))))))

(fn ConstructionScript)