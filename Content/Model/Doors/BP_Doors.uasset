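; BP_Doors is a double door that a VR player can open only while carrying a clip (GotAClip).
; Box overlap checks the VRPawn, showing either the prompt widget with input enabled or an error widget; leaving hides both and disables input.
; Either grab action shows a waiting indicator, then after a fixed delay timelines swing both doors open by yaw.
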(event OnComponentBeginOverlap(Box)
  (params (OverlappedComponent :type Primitive%20Component%20Object%20Reference) (OtherActor :type Actor%20Object%20Reference) (OtherComp :type Primitive%20Component%20Object%20Reference) (OtherBodyIndex :type Integer) (bFromSweep :type Boolean) (SweepResult :type Hit%20Result%20Structure%20%28by%20ref%29))
  (bind _widget (Variables|Default|GetWidget))
  (bind _error (Variables|Default|GetError))
  (bind _asvrpawn (Utilities|Casting|CastToVRPawn OtherActor))
  (if (Variables|/Game/VRTemplate/Blueprints/VRPawn.VRPawn_C|Getgot_a_clip? _asvrpawn)
    (Input|EnableInput (Game|GetPlayerController 0))
    (Rendering|SetVisibility _error false false)
    (Rendering|SetVisibility _widget true false)
    (else
      (Rendering|SetVisibility _error true false)
      (Rendering|SetVisibility _widget false false))))

(event OnComponentEndOverlap(Box)
  (params (OverlappedComponent :type Primitive%20Component%20Object%20Reference) (OtherActor :type Actor%20Object%20Reference) (OtherComp :type Primitive%20Component%20Object%20Reference) (OtherBodyIndex :type Integer))
  (Utilities|Casting|CastToVRPawn OtherActor)
  (Input|DisableInput (Game|GetPlayerController 0))
  (Rendering|SetVisibility (Variables|Default|GetError) false false)
  (Rendering|SetVisibility (Variables|Default|GetWidget) false false))

(event Input|EnhancedActionEvents|EnhancedInputActionIA_Grab_Right
  (params (ActionValue :type Float%20%28double-precision%29) (ElapsedSeconds :type Float%20%28double-precision%29) (TriggeredSeconds :type Float%20%28double-precision%29) (InputAction :type Input%20Action%20Object%20Reference :default "/Game/VRTemplate/Input/Actions/IA_Grab_Right.IA_Grab_Right"))
  (:Started
    (Utilities|FlowControl|Delay 1e+01)
    (Rendering|SetVisibility (Variables|Default|GetWaiting) false false)
    (bind _rotate_z_right (Timeline|Right%20Door%20Rotate%20Timeline Play)
      (:Update
        (Transformation|SetRelativeRotation (Variables|Default|GetDoorRight) (Math|Rotator|MakeRotator 0.0 0.0 _rotate_z_right) false false)))))

(event Input|EnhancedActionEvents|EnhancedInputActionIA_Grab_Right
  (params (ActionValue :type Float%20%28double-precision%29) (ElapsedSeconds :type Float%20%28double-precision%29) (TriggeredSeconds :type Float%20%28double-precision%29) (InputAction :type Input%20Action%20Object%20Reference :default "/Game/VRTemplate/Input/Actions/IA_Grab_Right.IA_Grab_Right"))
  (:Started
    (Rendering|SetVisibility (Variables|Default|GetWidget) false false)
    (Rendering|SetVisibility (Variables|Default|GetWaiting) true false)
    (Utilities|FlowControl|Delay 1e+01)
    (bind _rotate_z_left (Timeline|Left%20Door%20Rotate%20Timeline Play)
      (:Update
        (Transformation|SetRelativeRotation (Variables|Default|GetDoorLeft) (Math|Rotator|MakeRotator 0.0 0.0 _rotate_z_left) false false)))))

(event Input|EnhancedActionEvents|EnhancedInputActionIA_Grab_Left
  (params (ActionValue :type Float%20%28double-precision%29) (ElapsedSeconds :type Float%20%28double-precision%29) (TriggeredSeconds :type Float%20%28double-precision%29) (InputAction :type Input%20Action%20Object%20Reference :default "/Game/VRTemplate/Input/Actions/IA_Grab_Left.IA_Grab_Left"))
  (:Started
    (Utilities|FlowControl|Delay 1e+01)
    (Rendering|SetVisibility (Variables|Default|GetWaiting) false false)
    (bind _rotate_z_right (Timeline|Right%20Door%20Rotate%20Timeline Play)
      (:Update
        (Transformation|SetRelativeRotation (Variables|Default|GetDoorRight) (Math|Rotator|MakeRotator 0.0 0.0 _rotate_z_right) false false)))))

(event Input|EnhancedActionEvents|EnhancedInputActionIA_Grab_Left
  (params (ActionValue :type Float%20%28double-precision%29) (ElapsedSeconds :type Float%20%28double-precision%29) (TriggeredSeconds :type Float%20%28double-precision%29) (InputAction :type Input%20Action%20Object%20Reference :default "/Game/VRTemplate/Input/Actions/IA_Grab_Left.IA_Grab_Left"))
  (:Started
    (Rendering|SetVisibility (Variables|Default|GetWidget) false false)
    (Rendering|SetVisibility (Variables|Default|GetWaiting) true false)
    (Utilities|FlowControl|Delay 1e+01)
    (bind _rotate_z_left (Timeline|Left%20Door%20Rotate%20Timeline Play)
      (:Update
        (Transformation|SetRelativeRotation (Variables|Default|GetDoorLeft) (Math|Rotator|MakeRotator 0.0 0.0 _rotate_z_left) false false)))))

(fn ConstructionScript)